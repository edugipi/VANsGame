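; CheckpointBP is a checkpoint trigger that saves progress when a VAN actor overlaps its Box component.
; It loads the MySaveGame from a fixed slot, or creates one if none exists, then stores the VAN's current location as LastCheckpointLocation.
; The save is written back to the slot and a debug message is printed; this Blueprint only saves and does not handle respawning.
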(event OnComponentBeginOverlap(Box)
  (params (OverlappedComponent :type Primitive%20Component%20Object%20Reference) (OtherActor :type Actor%20Object%20Reference) (OtherComp :type Primitive%20Component%20Object%20Reference) (OtherBodyIndex :type Integer) (bFromSweep :type Boolean) (SweepResult :type Hit%20Result%20Structure%20%28by%20ref%29))
  (bind _asvan (Utilities|Casting|CastToVAN OtherActor))
  (Variables|Default|SetLocation (Transformation|GetActorLocation _asvan))
  (bind _returnvalue (SaveGame|DoesSaveGameExist "SlotName"))
  (if _returnvalue
    (bind _returnvalue_2 (SaveGame|LoadGamefromSlot "SlotName"))
    (bind _output_get (Variables|Default|SetSaverSubClass _returnvalue_2))
    (bind _asmy_save_game (Utilities|Casting|CastToMySaveGame _output_get))
    (Variables|/Game/Saves_Checkpoints/MySaveGame.MySaveGame_C|SetLastCheckpointLocation _asmy_save_game (Variables|Default|GetLocation))
    (SaveGame|SaveGametoSlot (Variables|Default|GetSaverSubClass) "SlotName")
    (Development|PrintString "Checkpoint Save!")
    (else
      (bind _returnvalue_3 (SaveGame|CreateSaveGameObject "/Game/Saves_Checkpoints/MySaveGame.MySaveGame_C"))
      (bind _output_get_2 (Variables|Default|SetSaverSubClass _returnvalue_3))
      (bind _asmy_save_game_2 (Utilities|Casting|CastToMySaveGame _output_get_2))
      (Variables|/Game/Saves_Checkpoints/MySaveGame.MySaveGame_C|SetLastCheckpointLocation _asmy_save_game_2 (Variables|Default|GetLocation))
      (SaveGame|SaveGametoSlot (Variables|Default|GetSaverSubClass) "SlotName")
      (Development|PrintString "Checkpoint Save!"))))

(event EventBeginPlay)

(event Collision|EventActorBeginOverlap
  (params (OtherActor :type Actor%20Object%20Reference)))

(event EventTick
  (params (DeltaSeconds :type Float%20%28single-precision%29)))

(fn ConstructionScript)